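; Player Blueprint with a first-person camera that handles interacting with, holding and dropping items.
; The Interact input drops a held item, or otherwise triggers the Interacter component from the camera's position and forward vector.
; SetCurrentItem stores the item in Blueprint and C++-named variables, then a timeline lerps it toward the Hand.
; Dropping re-enables physics, detaches the item keeping world transform, and clears both references.
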(event `InputAction|Interact`
  (params (Key :type "Key Structure"))
  (bind _firstpersoncamera (`self.FirstPersonCamera`))
  (:`Pressed`
    (`/Engine/EditorBlueprintResources/StandardMacros.IsValid` (`self.CurrentHeldItem_0`)
      (:`Is Valid`
        (`self.RemoveCurrentItem`))
      (:`Is Not Valid`
        (`Interacter.TriggerInteract` (`self.Interacter`) (`SceneComponent.K2_GetComponentToWorld` _firstpersoncamera) (`SceneComponent.GetForwardVector` _firstpersoncamera))))))

(event `self.ReceiveBeginPlay`
  (set `self.HandRef` (`self.Hand`)))

(event `SetCurrentItem`
  (params (CurrentHeldIItem :type "StaticMeshComponent Object Reference"))
  (bind _currenthelditemcpp (`self.CurrentHeldItemCpp`))
  (bind _output_get (set `self.CurrentHeldItem_0` CurrentHeldIItem))
  (set `self.CurrentHeldItemCpp` _output_get)
  (bind (_direction _picktime) (`Timeline|PickItenTimeline` :!via `PlayFromStart`)
    (:`Update`
      (`/Engine/EditorBlueprintResources/StandardMacros.IsValid` (`self.CurrentHeldItemCpp`)
        (:`Is Valid`
          (`SceneComponent.K2_SetWorldLocation` _currenthelditemcpp (`KismetMathLibrary.VLerp` (`SceneComponent.K2_GetComponentLocation` _currenthelditemcpp) (`SceneComponent.K2_GetComponentLocation` (`self.Hand`)) _picktime) false false))))))

(event `RemoveCurrentItem`
  (bind _currenthelditem_0 (`self.CurrentHeldItem_0`))
  (`PrimitiveComponent.SetSimulatePhysics` _currenthelditem_0 true)
  (`SceneComponent.K2_DetachFromComponent` _currenthelditem_0 "KeepWorld" "KeepWorld" "KeepWorld" true)
  (set `self.CurrentHeldItem_0` null)
  ;[1 1 1] Bro!
  (set `self.CurrentHeldItemCpp` null))

(fn `UserConstructionScript`)