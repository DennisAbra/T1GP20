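; Manager actor that drives every BP_BlowTorch in the level from the bell ring event of a referenced Clock.
; On BeginPlay it binds to the Clock's bell event and caches all torch actors found in the world.
; Each ring increments a counter and passes it to every torch's BlowOutTorch, leaving each torch to act on the current ring number.
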(event `self.ReceiveBeginPlay`
  (add `/Game/Blueprints/GameMechanics/BP_MyClock.BellRingEvent` (`self.Clock`) (delegate `BellRinged`))
  (bind _outactors (`GameplayStatics.GetAllActorsOfClass` "/Game/Blueprints/BP_BlowTorch.BP_BlowTorch_C"))
  (set `self.BlowTorches` _outactors))

(event `BellRinged`
  (`/Engine/EditorBlueprintResources/StandardMacros.IncrementInt` (`self.CurrentRing`)
    (:`  `
      (for _array_element (`self.BlowTorches`)
        (`/Game/Blueprints/BP_BlowTorch.BlowOutTorch` _array_element (`self.CurrentRing`))))))

(fn `UserConstructionScript`)