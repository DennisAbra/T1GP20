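; BP_BrokenCoffin is an interactable broken coffin that plays voice-over lines with subtitles hinting that something is missing.
; Each permitted interaction increments a coffin counter on the game instance, which selects the line and resets upon reaching InteractMax.
; Playing a line blocks further interaction until the subtitle component signals that audio has finished and a delay has elapsed.
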(event `self.ReceiveBeginPlay`
  ;[1 1 1] Play Voice Over and Subtitles
  (add `/Game/Blueprints/GameMechanics/BP_Subtitle.CallAudioFinished` (`self.BP_Subtitle`) (delegate `CallAudioFinished_Event_0`))
  (bind _asbp_t1gp20game_instance (cast `/Game/Blueprints/Core/BP_T1GP20GameInstance` (`GameplayStatics.GetGameInstance`)))
  (set `self.RefToGameInstance` _asbp_t1gp20game_instance))

(event `CallAudioFinished_Event_0`
  ;[1 1 1] Play Voice Over and Subtitles
  (`KismetSystemLibrary.Delay` (`self.DelayDuration`))
  (set `self.CanInteract` true))

(event `self.Interact`
  (if (`self.CanInteract`)
    (bind _result (`/Engine/EditorBlueprintResources/StandardMacros.IncrementInt` (`/Game/Blueprints/Core/BP_T1GP20GameInstance.CoffinCounter` (`self.RefToGameInstance`)))
      (:`  `
        (`self.PlayVoiceOverAndSubtitles` _result)
        (if (== (`/Game/Blueprints/Core/BP_T1GP20GameInstance.CoffinCounter` (`self.RefToGameInstance`)) (`self.InteractMax`))
          (set `/Game/Blueprints/Core/BP_T1GP20GameInstance.CoffinCounter` 0 (`self.RefToGameInstance`)))))))

(fn `PlayVoiceOverAndSubtitles`
  (params (ActiveNo :type Integer))
  (bind _bp_subtitle (`self.BP_Subtitle`))
  (switch `int` ActiveNo
    (:`1`
      (`/Game/Blueprints/GameMechanics/BP_Subtitle.PlaySubtitle` _bp_subtitle "/Game/Sound/Tutorial/Coffin_-_I_must_be_missing_something_Cue.Coffin_-_I_must_be_missing_something_Cue" "I must be missing something"))
    (:`2`
      (`/Game/Blueprints/GameMechanics/BP_Subtitle.PlaySubtitle` _bp_subtitle "/Game/Sound/Tutorial/Coffin_-_There_seems_to_be_something_missing_Cue.Coffin_-_There_seems_to_be_something_missing_Cue" "There seems to be something missing")))
  (set `self.CanInteract` false))

(fn `UserConstructionScript`)