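; BP_DecalGroup is a decal Blueprint that stays hidden until a matching ring count triggers its fade-in.
; BeginPlay hides the Decal component.
; StartFadeIn compares the passed CurrentRingCount to OnRingOrder and, on an exact match, shows the decal and fades it in over FadeDuration with no delay.
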(event `self.ReceiveBeginPlay`
  (`SceneComponent.SetVisibility` (`self.Decal`) false false))

(event `StartFadeIn`
  (params (CurrentRingCount :type Integer))
  (if (== CurrentRingCount (`self.OnRingOrder`))
    (`SceneComponent.SetVisibility` (`self.Decal`) true false)
    (`DecalComponent.SetFadeIn` (`self.Decal`) 0.0 (`self.FadeDuration`))))

(fn `UserConstructionScript`)