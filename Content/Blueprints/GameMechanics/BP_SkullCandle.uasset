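; Skull candle puzzle piece that lights when an actor tagged Torch overlaps its collision volume.
; Lighting shows the idle particles, sets IsLit and registers the candle with its Manager along with its OrderToLightIn, for an ordered-lighting puzzle.
; BlowOutCandle hides the particles and clears IsLit.
; Interact only prints a placeholder for a puzzle clue.
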(event `self.Interact`
  (`KismetSystemLibrary.PrintString` "Input clue on how to solve puzzle here"))

(event `self.ReceiveBeginPlay`
  (`SceneComponent.SetVisibility` (`self.IdleParticlesComponent`) false false))

(event `self.CollisionVolume.OnComponentBeginOverlap`
  (params (OverlappedComponent :type "PrimitiveComponent Object Reference") (OtherActor :type "Actor Object Reference") (OtherComp :type "PrimitiveComponent Object Reference") (OtherBodyIndex :type Integer) (bFromSweep :type Boolean) (SweepResult :type "HitResult Structure (by ref)"))
  (if (`self.ActorHasTag` OtherActor "Torch")
    (set `self.bIsLit` true)
    (`KismetSystemLibrary.PrintString` "Light Candle")
    (`SceneComponent.SetVisibility` (`self.IdleParticlesComponent`) true false)
    (`/Game/Blueprints/GameMechanics/BP_SkullManager.RegisterCandle` (`self.Manager`) self (`self.OrderToLightIn`))))

(fn `BlowOutCandle`
  (`SceneComponent.SetVisibility` (`self.IdleParticlesComponent`) false false)
  (`KismetSystemLibrary.PrintString` "Candle was blown out")
  (set `self.bIsLit` false))

(fn `UserConstructionScript`
  (`parent.UserConstructionScript`))