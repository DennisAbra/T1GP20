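; BP_HoverBase is a hover base Blueprint with a Book component, apparently meant to bob and spin it.
; BeginPlay binds an empty handler to BPSubtitle's audio-finished event, caches the game instance and stores the Book's relative location.
; A timeline-driven vertical offset and a yaw rotation step are present but disconnected, so this graph never animates the Book.
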(event `self.ReceiveBeginPlay`
  (add `/Game/Blueprints/GameMechanics/BP_Subtitle.CallAudioFinished` (`self.BP_Subtitle`) (delegate `CallAudioFinished_Event_0`))
  (bind _asbp_t1gp20game_instance (cast `/Game/Blueprints/Core/BP_T1GP20GameInstance` (`GameplayStatics.GetGameInstance`)))
  (set `self.RefToGameInstance` _asbp_t1gp20game_instance)
  (set `self.PreSavedLocation` (`SceneComponent.RelativeLocation` (`self.Book`))))

(event `CallAudioFinished_Event_0`)

(fn `UserConstructionScript`)