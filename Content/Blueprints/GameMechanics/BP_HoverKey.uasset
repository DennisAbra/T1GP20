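; BP_HoverKey is an interactable that plays one of three spoken hint lines with subtitles about a book riddle.
; Each interaction increments KeyBookCounter on the game instance, plays the matching line through BPSubtitle and resets the counter when it reaches InteractMax.
; Playing a line clears CanInteract, and the audio-finished event restores it after a delay, so lines do not overlap.
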(event `self.Interact`
  (if (`self.CanInteract`)
    (bind _result (`/Engine/EditorBlueprintResources/StandardMacros.IncrementInt` (`/Game/Blueprints/Core/BP_T1GP20GameInstance.KeyBookCounter` (`self.RefToGameInstance`)))
      (:`  `
        (`self.PlayVoiceOverAndSubtitles` _result)
        (if (== (`/Game/Blueprints/Core/BP_T1GP20GameInstance.KeyBookCounter` (`self.RefToGameInstance`)) (`self.InteractMax`))
          (set `/Game/Blueprints/Core/BP_T1GP20GameInstance.KeyBookCounter` 0 (`self.RefToGameInstance`)))))))

(event `self.CallAudioFinished_Event_0`
  (`KismetSystemLibrary.Delay` (`self.DelayDuration`))
  (set `self.CanInteract` true))

(fn `PlayVoiceOverAndSubtitles`
  (params (ActiveNo :type Integer))
  (switch `int` ActiveNo
    (:`1`
      (`/Game/Blueprints/GameMechanics/BP_Subtitle.PlaySubtitle` (`self.BP_Subtitle`) "/Game/Sound/Tutorial/Book_-_I_wonder_what_it_could_mean_Cue.Book_-_I_wonder_what_it_could_mean_Cue" "I wonder what it could mean"))
    (:`2`
      (`/Game/Blueprints/GameMechanics/BP_Subtitle.PlaySubtitle` (`self.BP_Subtitle`) "/Game/Sound/Tutorial/Book_-_Maybe_this_is_a_riddle_Cue.Book_-_Maybe_this_is_a_riddle_Cue" "Maybe this is a riddle"))
    (:`3`
      (`/Game/Blueprints/GameMechanics/BP_Subtitle.PlaySubtitle` (`self.BP_Subtitle`) "/Game/Sound/Tutorial/Book_-_Should_be_some_item_Cue.Book_-_Should_be_some_item_Cue" "Should be some item")))
  (set `self.CanInteract` false))

(fn `UserConstructionScript`
  (`parent.UserConstructionScript`))