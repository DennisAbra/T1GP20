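; Jigsaw puzzle piece that the player carries and releases, snapping into its final spot when placed correctly.
; BeginPlay stores the FinalPosition marker's transform in the JigsawPiece component, which tests each drop.
; A correct drop disables physics, lerps the piece home by timeline, blocks re-interaction and has the manager check completion.
; Subtitled voice lines rotate through Game Instance counters for right and wrong drops, gated by playing audio and a cooldown.
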(event `self.ReceiveBeginPlay`
  ;[1 1 1] Setup
  (`parent.ReceiveBeginPlay`)
  (`SceneComponent.K2_DetachFromComponent` (`self.FinalPosition`) "KeepWorld" "KeepWorld" "KeepWorld" true)
  (`JigsawPieceComponent.SetFinalTransform` (`self.JigsawPiece`) (`SceneComponent.K2_GetComponentToWorld` (`self.FinalPosition`)))
  (set `self.bIsJigsaw` true)
  ;[1 1 1] BindEvent to audio finished and Get reference to Game Instance
  (add `/Game/Blueprints/GameMechanics/BP_Subtitle.CallAudioFinished` (`self.BP_Subtitle`) (delegate `CallAudioFinished_Event_0`))
  (bind _asbp_t1gp20game_instance (cast `/Game/Blueprints/Core/BP_T1GP20GameInstance` (`GameplayStatics.GetGameInstance`)))
  (set `self.RefToGameInstance` _asbp_t1gp20game_instance))

(event `CallAudioFinished_Event_0`
  ;[1 1 1] BindEvent to audio finished and Get reference to Game Instance
  (`KismetSystemLibrary.Delay` (`self.DelayDuration`))
  (set `self.CanInteract` true))

(event `self.Interact`
  (if (not (`self.bIsCorrect`))
    (`parent.Interact`)))

(event `self.DetachFromPlayer`
  (bind _objectmesh (`self.ObjectMesh`))
  (bind _objectmesh_2 (`self.ObjectMesh`))
  (`parent.DetachFromPlayer`)
  (bind _returnvalue (`JigsawPieceComponent.TestPosition` (`self.JigsawPiece`) (`SceneComponent.K2_GetComponentToWorld` (`self.ObjectMesh`))))
  (if _returnvalue
    (`PrimitiveComponent.SetSimulatePhysics` (`self.ObjectMesh`) false)
    (bind _returnvalue_2 (`JigsawPieceComponent.GetFinalTransform` (`self.JigsawPiece`)))
    (bind (_direction _loc) (`Timeline|LerpToFinal` :!via `PlayFromStart`)
      (:`Update`
        (`SceneComponent.K2_SetWorldLocation` _objectmesh_2 (`KismetMathLibrary.VLerp` (`SceneComponent.K2_GetComponentLocation` _objectmesh) (.location _returnvalue_2) _loc) false false)
        (`SceneComponent.K2_SetWorldRotation` _objectmesh_2 (`KismetMathLibrary.RLerp` (`SceneComponent.K2_GetComponentRotation` _objectmesh) (.rotation _returnvalue_2) _loc) false false))
      (:`Finished`
        (if (and (`self.CanInteract`) (not (`/Game/Blueprints/Core/BP_T1GP20GameInstance.VoiceIsPlaying` (`self.RefToGameInstance`))))
          (`self.Scenario1_InteractCountAndPlayAudio`))
        (set `self.bIsCorrect` true)
        (`/Game/Blueprints/GameMechanics/Jigsaw/BP_JigsawManager.CheckWinCondition` (`self.ManagerRef`))
        (`KismetSystemLibrary.Delay` 2.0)
        (if (`/Game/Blueprints/GameMechanics/Jigsaw/BP_JigsawManager.bPuzzleComplete` (`self.ManagerRef`))
          (`/Game/Blueprints/GameMechanics/BP_Subtitle.PlaySubtitle` (`self.BP_Subtitle`) "/Game/Sound/Tutorial/Coffin_-_Woah__Something_seems_to_have_happend_Cue.Coffin_-_Woah__Something_seems_to_have_happend_Cue" "Woah, something seems to have happend"))))
    (elif (and (`self.CanInteract`) (not (`/Game/Blueprints/Core/BP_T1GP20GameInstance.VoiceIsPlaying` (`self.RefToGameInstance`))))
      (`self.Scenario2_InteractCountAndPlayAudio`))))

(fn `Scenario1_InteractCountAndPlayAudio`
  (bind _result (`/Engine/EditorBlueprintResources/StandardMacros.IncrementInt` (`/Game/Blueprints/Core/BP_T1GP20GameInstance.JigsawCounterScenario1` (`self.RefToGameInstance`)))
    (:`  `
      (`self.Secenario1_PlayVoiceOverAndSubtitles` _result)
      (if (== (`/Game/Blueprints/Core/BP_T1GP20GameInstance.JigsawCounterScenario1` (`self.RefToGameInstance`)) (`self.InteractMax`))
        (set `/Game/Blueprints/Core/BP_T1GP20GameInstance.JigsawCounterScenario1` 0 (`self.RefToGameInstance`))))))

(fn `Scenario2_InteractCountAndPlayAudio`
  (bind _result (`/Engine/EditorBlueprintResources/StandardMacros.IncrementInt` (`/Game/Blueprints/Core/BP_T1GP20GameInstance.JigsawCounterScenario2` (`self.RefToGameInstance`)))
    (:`  `
      (`self.Scenario2_PlayVoiceOverAndSubtitles` _result)
      (if (== (`/Game/Blueprints/Core/BP_T1GP20GameInstance.JigsawCounterScenario2` (`self.RefToGameInstance`)) (`self.InteractMax`))
        (set `/Game/Blueprints/Core/BP_T1GP20GameInstance.JigsawCounterScenario2` 0 (`self.RefToGameInstance`))))))

(fn `Scenario2_PlayVoiceOverAndSubtitles`
  (params (ActiveNo :type Integer))
  (switch `int` ActiveNo
    (:`1`
      (`/Game/Blueprints/GameMechanics/BP_Subtitle.PlaySubtitle` (`self.BP_Subtitle`) "/Game/Sound/Tutorial/Coffin_-_This_does_not_seem_to_fit_here_Cue.Coffin_-_This_does_not_seem_to_fit_here_Cue" "This does not seem to fit here"))
    (:`2`
      (`/Game/Blueprints/GameMechanics/BP_Subtitle.PlaySubtitle` (`self.BP_Subtitle`) "/Game/Sound/Tutorial/Coffin_-_There_seems_to_be_something_missing_Cue.Coffin_-_There_seems_to_be_something_missing_Cue" "It looks like there is something missing")))
  (set `self.CanInteract` false))

(fn `Secenario1_PlayVoiceOverAndSubtitles`
  (params (ActiveNo :type Integer))
  (bind _bp_subtitle (`self.BP_Subtitle`))
  (switch `int` ActiveNo
    (:`1`
      (`/Game/Blueprints/GameMechanics/BP_Subtitle.PlaySubtitle` _bp_subtitle "/Game/Sound/Tutorial/Coffin_-_That_seemed_to_work_Cue.Coffin_-_That_seemed_to_work_Cue" "That seemed to work"))
    (:`2`
      (`/Game/Blueprints/GameMechanics/BP_Subtitle.PlaySubtitle` _bp_subtitle "/Game/Sound/Tutorial/Coffin_-_That_did_it_Cue.Coffin_-_That_did_it_Cue" "That did it")))
  (set `self.CanInteract` false))

(fn `UserConstructionScript`
  (`parent.UserConstructionScript`))