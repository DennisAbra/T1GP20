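; Jigsaw puzzle manager that tracks correctly placed pieces and unlocks a gate button when the puzzle is solved.
; Each CheckWinCondition call increments a counter, which starts at zero on BeginPlay, and compares it to MaxPuzzlePieces.
; On a match, it waits briefly and activates the referenced GateButton through SetPuzzleActivate, if that button is valid.
; Win and no-win states are reported only through debug print strings.
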(event `self.ReceiveBeginPlay`
  (set `self.CorrectlyPlacedCounter` 0))

(event `CheckWinCondition`
  (`/Engine/EditorBlueprintResources/StandardMacros.IncrementInt` (`self.CorrectlyPlacedCounter`)
    (:`  `
      (if (== (`self.MaxPuzzlePieces`) (`self.CorrectlyPlacedCounter`))
        (`KismetSystemLibrary.PrintString` "WON THE GAME")
        (bind _gatebutton (`self.GateButton`)
          (:`then`
            (`KismetSystemLibrary.Delay` 1.0)
            (`PearlGateButton.SetPuzzleActivate` _gatebutton true))
          (:`else`))
        (else
          (`KismetSystemLibrary.PrintString` "NO WIN YET"))))))

(fn `UserConstructionScript`)