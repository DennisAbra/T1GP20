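; BP_Subtitle plays voice or sound cues in 2D with optional on-screen subtitle text.
; On BeginPlay it creates a WBP_Tutorial widget and caches the game instance, which holds the ShowSubittles setting.
; PlaySubtitle spawns the sound and, if that setting is on, shows the text for DelayDuration, independent of audio length.
; When the audio finishes, it fires the CallAudioFinished dispatcher.
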(event `self.ReceiveBeginPlay`
  (bind _returnvalue (`|CreateWidget` "/Game/UI/WBP_Tutorial.WBP_Tutorial_C"))
  (bind _output_get (set `self.TutorialWidget` _returnvalue))
  (`UserWidget.AddToViewport` _output_get 0)
  (bind _asbp_t1gp20game_instance (cast `/Game/Blueprints/Core/BP_T1GP20GameInstance` (`GameplayStatics.GetGameInstance`)))
  (bind _output_get_2 (set `self.RefToGameInstance` _asbp_t1gp20game_instance))
  (set `self.ShouldShowSubtitle` (`/Game/Blueprints/Core/BP_T1GP20GameInstance.ShowSubittles` _output_get_2)))

(event `PlaySubtitle`
  (params (SoundCue :type "SoundCue Object Reference") (Subtitle :type Text))
  (bind _returnvalue (`GameplayStatics.SpawnSound2D` SoundCue 1.0 1.0 0.0 null))
  (add `AudioComponent.OnAudioFinished` _returnvalue (delegate `AudioFinished`))
  (if (`/Game/Blueprints/Core/BP_T1GP20GameInstance.ShowSubittles` (`self.RefToGameInstance`))
    (`TextBlock.SetText` (`/Game/UI/WBP_Tutorial.Display_Text` (`self.TutorialWidget`)) Subtitle)
    (`/Game/UI/WBP_Tutorial.Visible` (`self.TutorialWidget`))
    (`KismetSystemLibrary.Delay` (`self.Delay Duration`))
    (`/Game/UI/WBP_Tutorial.Invisible` (`self.TutorialWidget`))))

(event `AudioFinished`
  (`self.CallAudioFinished`))