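; BP_SkullManager runs an ordered candle-lighting puzzle, tracking the expected order and completion state.
; RegisterCandle stores each candle, waits WaitTime, then compares its order to CurrentOrder, advancing on a match and finishing when the counter reaches MaxAmountOfCandles.
; A wrong order blows out every stored candle, clears the list and resets the sequence.
; Completion only sets a flag and prints a message, after which registrations are ignored.
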(event `self.ReceiveBeginPlay`
  (set `self.CurrentOrder` 1))

(event `RegisterCandle`
  (params (CandleToRegister :type "/Game/Blueprints/GameMechanics/BP_SkullCandle Object Reference") (OrderToLightIn :type Integer))
  (bind _candles (`self.Candles`))
  (if (`self.bFinishedPuzzle`)
    (`KismetSystemLibrary.PrintString` "Puzzle Finished. Functionality turned off")
    (else
      (`KismetArrayLibrary.Array_Add` (`self.Candles`) CandleToRegister)
      (`KismetSystemLibrary.Delay` (`self.WaitTime`))
      ;[1 1 1] Add Timer before this to delay the candle being blown out
      (if (== OrderToLightIn (`self.CurrentOrder`))
        (`KismetSystemLibrary.PrintString` "Let it be lit")
        (bind _result (`/Engine/EditorBlueprintResources/StandardMacros.IncrementInt` (`self.CurrentOrder`))
          (:`  `
            (if (== _result (`self.MaxAmountOfCandles`))
              (`KismetSystemLibrary.PrintString` "PUZZLE COMPLETE")
              (set `self.bFinishedPuzzle` true))))
        (else
          (`KismetSystemLibrary.PrintString` "BLOW OUT")
          (for _array_element _candles
            (`/Game/Blueprints/GameMechanics/BP_SkullCandle.BlowOutCandle` _array_element))
          (set `self.CurrentOrder` 1)
          (`KismetArrayLibrary.Array_Clear` _candles))))))

(fn `UserConstructionScript`)