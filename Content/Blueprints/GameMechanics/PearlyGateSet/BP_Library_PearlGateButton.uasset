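; BP_Library_PearlGateButton is a rotatable puzzle disc that feeds the Pearly Gate lock.
; While rotated, a camera line trace and mouse delta go through C++ helpers to turn the disc, signal PearlGateLock and fade the rolling sound with mouse movement.
; TurnOnLight lights the spotlight, activates the puzzle and plays the angel animation.
; Interacting while inactive cycles voice-over subtitles using a GameInstance counter, gated until playback ends plus a delay.
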(event `self.RotateObject`
  (bind _audio (`self.Audio`))
  (bind (_deltax _deltay) (`PlayerController.GetInputMouseDelta` (`GameplayStatics.GetPlayerController` 0)))
  (bind (_deltax_2 _deltay_2) (`PlayerController.GetInputMouseDelta` (`GameplayStatics.GetPlayerController` 0)))
  (bind _returnvalue (`SceneComponent.K2_GetComponentLocation` (`FirstPersonController.FirstPersonCamera` (`self.Player`))))
  ;[0.6614 1 0.565] Play rolling disc sound
  (if (`ActorComponent.IsActive` _audio)
    (if (and (== _deltax_2 0.0) (== _deltay_2 0.0))
      (`AudioComponent.AdjustVolume` (`self.Audio`) 0.3 0.0 "Linear" :!label _label)
      (else
        (`AudioComponent.AdjustVolume` (`self.Audio`) 0.5 1.0 "Linear")
        ;[1 1 1] Rotate puzzle disc according to mouse value (position)
        (bind (_outhit _returnvalue_2) (`KismetSystemLibrary.LineTraceSingle` :`Start` _returnvalue :`End` (+ _returnvalue (* (`SceneComponent.GetForwardVector` (`FirstPersonController.FirstPersonCamera` (`self.Player`))) (`self.RayTraceLength`))) :`TraceChannel` "TraceTypeQuery3" :`DrawDebugType` "ForOneFrame" :`bIgnoreSelf` false :`TraceColor` (struct :`R` 1.0 :`G` 0.135668 :`B` 0.847283 :`A` 1.0)))
        (if _returnvalue_2
          ;;[1 0.5728 0.8932 1 14] C++ code, get mouse position according to ray cast hit point
          (bind _returnvalue_3 (`self.GetRotationIncrement` (`self.FaceDirection`) (- (`.ImpactPoint` (`GameplayStatics.BreakHitResult` _outhit)) (`SceneComponent.K2_GetComponentLocation` (`self.PuzzleButton`))) (`KismetMathLibrary.MakeVector2D` _deltax _deltay)))
          (`SceneComponent.K2_AddLocalRotation` (`self.PuzzleButton`) (`KismetMathLibrary.MakeRotator` (* (`KismetMathLibrary.Conv_IntToDouble` _returnvalue_3) (`self.Speed`))) false false)
          ;;[1 0.5865 0.8685 1 14] C++ code, send rotation value to PearlGateLock
          (`self.EmitRotationSignal`))))
    (else
      (`ActorComponent.SetActive` _audio true false))))

(event `self.IsNotInteracting`
  ;[0.6614 1 0.565] Play rolling disc sound
  (goto _label))

(event `self.InteractWhenNotActivate`
  ;[1 0.9513 0.5229] Play voice over and subtitles
  (if (and (`self.CanInteract`) (not (`/Game/Blueprints/Core/BP_T1GP20GameInstance.VoiceIsPlaying` (`self.RefToGameInstance`))))
    (bind _result (`/Engine/EditorBlueprintResources/StandardMacros.IncrementInt` (`/Game/Blueprints/Core/BP_T1GP20GameInstance.StatueCoutner` (`self.RefToGameInstance`)))
      (:`  `
        (`self.PlayVoiceOverAndSubtitles` _result)
        (if (== (`/Game/Blueprints/Core/BP_T1GP20GameInstance.StatueCoutner` (`self.RefToGameInstance`)) (`self.InteractMax`))
          (set `/Game/Blueprints/Core/BP_T1GP20GameInstance.StatueCoutner` 0 (`self.RefToGameInstance`)))))))

(event `self.ReceiveBeginPlay`
  (`SceneComponent.SetVisibility` (`self.SpotLight`) false false)
  ;[1 0.9513 0.5229] Bind event and Get reference to Game Instance
  (add `/Game/Blueprints/GameMechanics/BP_Subtitle.CallAudioFinished` (`self.BP_Subtitle`) (delegate `CallAudioFinished_Event_0`))
  (bind _asbp_t1gp20game_instance (cast `/Game/Blueprints/Core/BP_T1GP20GameInstance` (`GameplayStatics.GetGameInstance`)))
  (set `self.RefToGameInstance` _asbp_t1gp20game_instance))

(event `CallAudioFinished_Event_0`
  ;[1 0.9513 0.5229] Bind event and Get reference to Game Instance
  (`KismetSystemLibrary.Delay` (`self.DelayDuration`))
  (set `self.CanInteract` true))

(event `TurnOnLight`
  (`SceneComponent.SetVisibility` (`self.SpotLight`) true false)
  (`self.SetPuzzleActivate` true)
  (`SkeletalMeshComponent.Play` (`self.AngelSkeletal`) false))

(fn `PlayVoiceOverAndSubtitles`
  (params (ActiveNo :type Integer))
  (switch `int` ActiveNo
    (:`1`
      (`/Game/Blueprints/GameMechanics/BP_Subtitle.PlaySubtitle` (`self.BP_Subtitle`) "/Game/Sound/Tutorial/Statue_-_I_can_t_access_this_Cue.Statue_-_I_can_t_access_this_Cue" "I can't access that"))
    (:`2`
      (`/Game/Blueprints/GameMechanics/BP_Subtitle.PlaySubtitle` (`self.BP_Subtitle`) "/Game/Sound/Tutorial/Statue_-_I_can_t_reach_that_Cue.Statue_-_I_can_t_reach_that_Cue" "I can't reach that")))
  (set `self.CanInteract` false))

(fn `UserConstructionScript`)