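; Rotatable button for the Pearl Gate puzzle that the player turns with mouse movement.
; RotateObject line-traces from the first-person camera and converts the hit offset and mouse delta into a yaw increment on PuzzleButton, then emits a rotation signal and plays a rolling sound.
; The sound stops when the mouse X and Y deltas are equal, as when idle.
; CheckMousePosition is unfinished and always returns false.
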(event `self.RotateObject`
  (bind (_deltax _deltay) (`PlayerController.GetInputMouseDelta` (`GameplayStatics.GetPlayerController` 0)))
  (bind (_deltax_2 _deltay_2) (`PlayerController.GetInputMouseDelta` (`GameplayStatics.GetPlayerController` 0)))
  (bind _returnvalue (`SceneComponent.K2_GetComponentLocation` (`FirstPersonController.FirstPersonCamera` (`self.Player`))))
  (if (!= _deltax_2 _deltay_2)
    (bind (_outhit _returnvalue_2) (`KismetSystemLibrary.LineTraceSingle` :`Start` _returnvalue :`End` (+ _returnvalue (* (`SceneComponent.GetForwardVector` (`FirstPersonController.FirstPersonCamera` (`self.Player`))) 500.0)) :`TraceChannel` "TraceTypeQuery3" :`DrawDebugType` "ForOneFrame" :`bIgnoreSelf` false :`TraceColor` (struct :`R` 1.0 :`G` 0.135668 :`B` 0.847283 :`A` 1.0)))
    (if _returnvalue_2
      (bind _returnvalue_3 (`self.GetRotationIncrement` (`self.FaceDirection`) (- (`.ImpactPoint` (`GameplayStatics.BreakHitResult` _outhit)) (`SceneComponent.K2_GetComponentLocation` (`self.PuzzleButton`))) (`KismetMathLibrary.MakeVector2D` _deltax _deltay)))
      (`SceneComponent.K2_AddLocalRotation` (`self.PuzzleButton`) (`KismetMathLibrary.MakeRotator` 0.0 0.0 (`KismetMathLibrary.Conv_IntToDouble` _returnvalue_3)) false false)
      (`self.EmitRotationSignal`)
      (`self.PlayRollingSound`))
    (else
      (`self.StopPlayRollingSound`))))

(fn `Check Mouse Position`
  (returns (bool :type Boolean))
  (bind _returnvalue (`WidgetLayoutLibrary.GetMousePositionOnPlatform`))
  (return false))

(fn `UserConstructionScript`)