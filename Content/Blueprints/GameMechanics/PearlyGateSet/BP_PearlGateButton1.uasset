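; Pearly gate puzzle button Blueprint, apparently meant to be rotated by mouse movement, but currently unfinished and inactive.
; RotateObject and MouseRedirection are empty events, and CheckMousePosition always returns false.
; Disconnected draft logic line-traces from the player's first-person camera to store a reference point, then on horizontal mouse movement yaws PuzzleButton toward the trace-derived angle using Atan2 and RInterpTo.
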(event `self.RotateObject`)

(event `self.MouseRedirection`)

(fn `Check Mouse Position`
  (returns (bool :type Boolean))
  (bind _returnvalue (`WidgetLayoutLibrary.GetMousePositionOnPlatform`))
  (return false))

(fn `UserConstructionScript`)