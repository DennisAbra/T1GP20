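; Base pearl gate puzzle button that plays hint voice lines with subtitles when interacted with while not activated.
; A counter on the game instance selects the line and resets at InteractMax, provided no other voice is playing.
; Interaction locks after a line and unlocks after a delay once BPSubtitle reports audio finished.
; RotateObject is empty and the mouse-driven trace rotation is unwired, while IsNotInteracting fades the audio out.
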(event `self.ReceiveBeginPlay`
  (add `/Game/Blueprints/GameMechanics/BP_Subtitle.CallAudioFinished` (`self.BP_Subtitle`) (delegate `CallAudioFinished_Event_0`))
  (bind _asbp_t1gp20game_instance (cast `/Game/Blueprints/Core/BP_T1GP20GameInstance` (`GameplayStatics.GetGameInstance`)))
  (set `self.RefToGameInstance` _asbp_t1gp20game_instance))

(event `CallAudioFinished_Event_0`
  (`KismetSystemLibrary.Delay` (`self.DelayDuration`))
  (set `self.CanInteract` true))

(event `self.InteractWhenNotActivate`
  (if (and (`self.CanInteract`) (not (`/Game/Blueprints/Core/BP_T1GP20GameInstance.VoiceIsPlaying` (`self.RefToGameInstance`))))
    (bind _result (`/Engine/EditorBlueprintResources/StandardMacros.IncrementInt` (`/Game/Blueprints/Core/BP_T1GP20GameInstance.StatueCoutner` (`self.RefToGameInstance`)))
      (:`  `
        (`self.PlayVoiceOverAndSubtitles` _result)
        (if (== (`/Game/Blueprints/Core/BP_T1GP20GameInstance.StatueCoutner` (`self.RefToGameInstance`)) (`self.InteractMax`))
          (set `/Game/Blueprints/Core/BP_T1GP20GameInstance.StatueCoutner` 0 (`self.RefToGameInstance`)))))))

(event `self.RotateObject`)

(event `self.IsNotInteracting`
  (`AudioComponent.AdjustVolume` (`self.Audio`) 0.3 0.0 "Linear"))

(fn `PlayVoiceOverAndSubtitles`
  (params (ActiveNo :type Integer))
  (switch `int` ActiveNo
    (:`1`
      (`/Game/Blueprints/GameMechanics/BP_Subtitle.PlaySubtitle` (`self.BP_Subtitle`) "/Game/Sound/Tutorial/Book_-_I_wonder_what_it_could_mean_Cue.Book_-_I_wonder_what_it_could_mean_Cue" "I wonder what it could mean"))
    (:`2`
      (`/Game/Blueprints/GameMechanics/BP_Subtitle.PlaySubtitle` (`self.BP_Subtitle`) "/Game/Sound/Tutorial/Book_-_Maybe_this_is_a_riddle_Cue.Book_-_Maybe_this_is_a_riddle_Cue" "Maybe this is a riddle"))
    (:`3`
      (`/Game/Blueprints/GameMechanics/BP_Subtitle.PlaySubtitle` (`self.BP_Subtitle`) "/Game/Sound/Tutorial/Book_-_Should_be_some_item_Cue.Book_-_Should_be_some_item_Cue" "Should be some item")))
  (set `self.CanInteract` false))

(fn `UserConstructionScript`)