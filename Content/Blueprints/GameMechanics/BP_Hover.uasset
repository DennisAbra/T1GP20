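; BP_Hover is a Blueprint with a Book component, set up for a hover-and-spin effect that is currently not wired to run.
; BeginPlay only saves the Book's starting relative location.
; Unreached nodes would offset that location vertically by a Timeline track scaled by HightVariation, and yaw the Book by RotationRate, but nothing triggers either.
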(event `self.ReceiveBeginPlay`
  (set `self.PreSavedLocation` (`SceneComponent.RelativeLocation` (`self.Book`))))

(fn `UserConstructionScript`)