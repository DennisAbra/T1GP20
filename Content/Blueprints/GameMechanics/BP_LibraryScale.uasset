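; Library scale puzzle prop with two trigger volumes: one checks the item placed on it, the other checks weight.
; Leaving either trigger calls TryCallUntrigger; both check results lead to no further action in this graph.
; Interacting plays one of three subtitled voice hints, cycled by a GameInstance counter that resets at InteractMax.
; A highlight event turns on the PearlGateButton light.
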(event `self.ReceiveBeginPlay`
  (bind _asbp_t1gp20game_instance (cast `/Game/Blueprints/Core/BP_T1GP20GameInstance` (`GameplayStatics.GetGameInstance`)))
  (set `self.RefToGameInstance` _asbp_t1gp20game_instance))

(event `self.Interact`
  (bind _result (`/Engine/EditorBlueprintResources/StandardMacros.IncrementInt` (`/Game/Blueprints/Core/BP_T1GP20GameInstance.ScaleCounter` (`self.RefToGameInstance`)))
    (:`  `
      (`self.PlayVoiceOverAndSubtitles` _result)
      (if (== (`/Game/Blueprints/Core/BP_T1GP20GameInstance.ScaleCounter` (`self.RefToGameInstance`)) (`self.InteractMax`))
        (set `/Game/Blueprints/Core/BP_T1GP20GameInstance.ScaleCounter` 0 (`self.RefToGameInstance`))))))

(event `self.ScaleTrigger1.OnComponentBeginOverlap`
  (params (OverlappedComponent :type "PrimitiveComponent Object Reference") (OtherActor :type "Actor Object Reference") (OtherComp :type "PrimitiveComponent Object Reference") (OtherBodyIndex :type Integer) (bFromSweep :type Boolean) (SweepResult :type "HitResult Structure (by ref)"))
  (bind _returnvalue (`self.CheckItem` OtherActor))
  (if _returnvalue
    _))

(event `self.ScaleTrigger1.OnComponentEndOverlap`
  (params (OverlappedComponent :type "PrimitiveComponent Object Reference") (OtherActor :type "Actor Object Reference") (OtherComp :type "PrimitiveComponent Object Reference") (OtherBodyIndex :type Integer))
  (`self.TryCallUntrigger` OtherActor))

(event `self.ScaleTrigger2.OnComponentBeginOverlap`
  (params (OverlappedComponent :type "PrimitiveComponent Object Reference") (OtherActor :type "Actor Object Reference") (OtherComp :type "PrimitiveComponent Object Reference") (OtherBodyIndex :type Integer) (bFromSweep :type Boolean) (SweepResult :type "HitResult Structure (by ref)"))
  (bind _returnvalue (`self.CheckWeight` OtherActor))
  (if _returnvalue
    _))

(event `self.ScaleTrigger2.OnComponentEndOverlap`
  (params (OverlappedComponent :type "PrimitiveComponent Object Reference") (OtherActor :type "Actor Object Reference") (OtherComp :type "PrimitiveComponent Object Reference") (OtherBodyIndex :type Integer))
  (`self.TryCallUntrigger` OtherActor))

(event `self.TurnOnHighlight`
  (`/Game/Blueprints/GameMechanics/PearlyGateSet/BP_Library_PearlGateButton.TurnOnLight` (`self.PearlGateButton`)))

(fn `PlayVoiceOverAndSubtitles`
  (params (ActiveNo :type Integer))
  (switch `int` ActiveNo
    (:`1`
      (`/Game/Blueprints/GameMechanics/BP_Subtitle.PlaySubtitle` (`self.BP_Subtitle`) "/Game/Sound/Tutorial/Scale_-_I_wonder_what_would_happen_if_I_put_something_on_the_scale_Cue.Scale_-_I_wonder_what_would_happen_if_I_put_something_on_the_scale_Cue" (0.0 0.0 0.0) "I wonder what would happen if i put something on the scale"))
    (:`2`
      (`/Game/Blueprints/GameMechanics/BP_Subtitle.PlaySubtitle` (`self.BP_Subtitle`) "/Game/Sound/Tutorial/Scale_-_I_should_try_and_put_something_on_the_scale_Cue.Scale_-_I_should_try_and_put_something_on_the_scale_Cue" (0.0 0.0 0.0) "I should try putting something on the scale"))
    (:`3`
      (`/Game/Blueprints/GameMechanics/BP_Subtitle.PlaySubtitle` (`self.BP_Subtitle`) "/Game/Sound/Tutorial/Scale_-_Maybe_I_should_weigh_something_Cue.Scale_-_Maybe_I_should_weigh_something_Cue" (0.0 0.0 0.0) "Maybe i should weigh something"))))

(fn `UserConstructionScript`)