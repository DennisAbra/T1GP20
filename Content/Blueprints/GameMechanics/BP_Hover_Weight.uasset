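; BP_Hover_Weight is an interactable book that shows a different subtitle on successive interactions.
; Interact increments WeightBookCounter on the Game Instance, so progress lives outside the actor, and resets it upon reaching InteractMax.
; PlayVoiceOverAndSubtitles maps the count to one of two placeholder-style lines, played through BPSubtitle at the book's location.
; Despite the function's name, only subtitle calls are present.
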(event `self.Interact`
  (bind _result (`/Engine/EditorBlueprintResources/StandardMacros.IncrementInt` (`/Game/Blueprints/Core/BP_T1GP20GameInstance.WeightBookCounter` (`self.RefToGameInstance`)))
    (:`  `
      (`self.PlayVoiceOverAndSubtitles` _result)
      (if (== (`/Game/Blueprints/Core/BP_T1GP20GameInstance.WeightBookCounter` (`self.RefToGameInstance`)) (`self.InteractMax`))
        (set `/Game/Blueprints/Core/BP_T1GP20GameInstance.WeightBookCounter` 0 (`self.RefToGameInstance`))))))

(fn `PlayVoiceOverAndSubtitles`
  (params (ActiveNo :type Integer))
  (switch `int` ActiveNo
    (:`1`
      (`/Game/Blueprints/GameMechanics/BP_Subtitle.PlaySubtitle` (`self.BP_Subtitle`) null (`SceneComponent.K2_GetComponentLocation` (`self.Book`)) "Something about color"))
    (:`2`
      (`/Game/Blueprints/GameMechanics/BP_Subtitle.PlaySubtitle` (`self.BP_Subtitle`) null (`SceneComponent.K2_GetComponentLocation` (`self.Book`)) "Something about weight"))))

(fn `UserConstructionScript`
  (`parent.UserConstructionScript`))