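; BP_SkullManager runs a sacrificial skull puzzle in which candles must be lit in a set order.
; Candles report to RegisterCandle with their order index, which is checked against a running counter; a wrong one blows out all registered candles after a delay and resets progress.
; Completing the sequence locks the puzzle and, if a GateButton is valid, activates it and reveals the hidden Pentagram after a short delay.
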(event `self.ReceiveBeginPlay`
  (set `self.CurrentOrder` 0)
  (`SceneComponent.SetVisibility` (`StaticMeshActor.StaticMeshComponent` (`self.Pentagram`)) false false))

(event `RegisterCandle`
  (params (CandleToRegister :type "/Game/Blueprints/GameMechanics/SkullPuzzle/BP_SkullCandle Object Reference") (OrderToLightIn :type Integer))
  (bind _candles (`self.Candles`))
  (bind _gatebutton (`self.GateButton`))
  (if (`self.bFinishedPuzzle`)
    (`KismetSystemLibrary.PrintString` "Puzzle Finished. Functionality turned off")
    (else
      (`KismetArrayLibrary.Array_Add` (`self.Candles`) CandleToRegister)
      (if (== OrderToLightIn (`self.CurrentOrder`))
        (bind _result (`/Engine/EditorBlueprintResources/StandardMacros.IncrementInt` (`self.CurrentOrder`))
          (:`  `
            (if (== _result (`self.MaxAmountOfCandles`))
              (`KismetSystemLibrary.PrintString` "PUZZLE COMPLETE")
              (set `self.bFinishedPuzzle` true)
              (`/Engine/EditorBlueprintResources/StandardMacros.IsValid` _gatebutton
                (:`Is Valid`
                  (`KismetSystemLibrary.Delay` 1.0)
                  (`PearlGateButton.SetPuzzleActivate` _gatebutton true)
                  (`SceneComponent.SetVisibility` (`StaticMeshActor.StaticMeshComponent` (`self.Pentagram`)) true false))))))
        (else
          (`KismetSystemLibrary.Delay` (`self.WaitTime`))
          (`KismetSystemLibrary.PrintString` "BLOW OUT")
          (for _array_element _candles
            (`/Game/Blueprints/GameMechanics/SkullPuzzle/BP_SkullCandle.BlowOutCandle` _array_element))
          (set `self.CurrentOrder` 0)
          (`KismetArrayLibrary.Array_Clear` _candles))))))

(fn `UserConstructionScript`)