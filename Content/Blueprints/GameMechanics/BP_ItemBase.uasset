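; Base item Blueprint for physics objects the player can pick up, carry and drop.
; Interact disables physics and Pawn/WorldStatic collision, attaches the mesh to the player's HandRef and registers it as the current item.
; DetachFromPlayer restores physics and collision and releases the mesh.
; Sufficiently fast hits play an impact sound chosen by MaterialInt, throttled by a DoOnce that resets after a short delay.
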(event `self.ReceiveHit`
  (params (MyComp :type "PrimitiveComponent Object Reference") (Other :type "Actor Object Reference") (OtherComp :type "PrimitiveComponent Object Reference") (bSelfMoved :type Boolean) (HitLocation :type "Vector Structure") (HitNormal :type "Vector Structure") (NormalImpulse :type "Vector Structure") (Hit :type "HitResult Structure (by ref)"))
  ;[0.7559 1 0.7958] Sound on drop thing
  (if (> (`KismetMathLibrary.VSize` (`SceneComponent.GetComponentVelocity` MyComp)) 65.0)
    (`/Engine/EditorBlueprintResources/StandardMacros.DoOnce` false :!label _label
      (:`Completed`
        (`GameplayStatics.PlaySoundAtLocation` (select `int` (`self.materialInt`) :`0` "/Game/Sound/PlayerSounds/Footsteps/FootstepCueBoot.FootstepCueBoot" :`1` "/Game/Sound/ItemSound/Thuds/Wood_thud_Cue.Wood_thud_Cue" :`2` "/Game/Sound/ItemSound/Thuds/Glass_thud_Cue.Glass_thud_Cue" :`3` "/Game/Sound/ItemSound/Thuds/GlassBreak_thud_Cue.GlassBreak_thud_Cue" :`4` "/Game/Sound/ItemSound/Thuds/Rock_thud_cue.Rock_thud_cue" :`5` "/Game/Sound/ItemSound/Thuds/SuperHeavyMetal_thud_Cue.SuperHeavyMetal_thud_Cue" :`6` "/Game/Sound/ItemSound/Thuds/Bone_thud_cue1.Bone_thud_cue1" :`7` "/Game/Sound/ItemSound/Thuds/Anchor_thud_cue.Anchor_thud_cue" :`8` "/Game/Sound/ItemSound/Thuds/Book_thud_cue.Book_thud_cue" :!type "SoundBase Object Reference") (`SceneComponent.K2_GetComponentLocation` MyComp) (struct) 1.0 1.0 0.0 null null null)
        (`KismetSystemLibrary.Delay` 0.2)
        (goto _label :!via `Reset`)))))

(event `self.ReceiveBeginPlay`
  (bind _asbp_player (cast `/Game/BP_Player` (`GameplayStatics.GetPlayerCharacter` 0)))
  (set `self.PlayerRef` _asbp_player))

(event `self.Interact`
  (bind _objectmesh (`self.ObjectMesh`))
  (bind _objectmesh_2 (`self.ObjectMesh`))
  ;[1 1 1] Attach To player
  (`PrimitiveComponent.SetSimulatePhysics` (`self.ObjectMesh`) false)
  (`PrimitiveComponent.SetCollisionResponseToChannel` _objectmesh_2 "ECC_Pawn" "ECR_Ignore")
  (`PrimitiveComponent.SetCollisionResponseToChannel` _objectmesh_2 "ECC_WorldStatic" "ECR_Ignore")
  (`SceneComponent.K2_AttachToComponent` _objectmesh (`/Game/BP_Player.HandRef` (`self.PlayerRef`)) "None" "KeepWorld" "KeepWorld" "KeepWorld" true)
  (set `self.bIsPickedUp` true)
  (`/Game/BP_Player.SetCurrentItem` (`self.PlayerRef`) _objectmesh)
  (`GameplayStatics.PlaySoundAtLocation` "/Game/Sound/PlayerSounds/Pickupsound_Cue.Pickupsound_Cue" (0.0 0.0 0.0) (struct) 1.0 1.0 0.0 null null null))

(event `DetachFromPlayer`
  (bind _objectmesh (`self.ObjectMesh`))
  (`PrimitiveComponent.SetSimulatePhysics` (`self.ObjectMesh`) true)
  (`SceneComponent.K2_DetachFromComponent` (`self.ObjectMesh`) "KeepWorld" "KeepWorld" "KeepWorld" true)
  (set `self.bIsPickedUp` false)
  (`PrimitiveComponent.SetCollisionResponseToChannel` _objectmesh "ECC_Pawn" "ECR_Block")
  (`PrimitiveComponent.SetCollisionResponseToChannel` _objectmesh "ECC_WorldStatic" "ECR_Block"))

(fn `UserConstructionScript`)