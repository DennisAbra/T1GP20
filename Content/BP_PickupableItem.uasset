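; BP_PickupableItem is a world item the player can pick up and drop through an Interact event.
; Interacting while loose turns off physics on the Cube and attaches it to the player ThirdPersonCharacter's HandRef, keeping its world transform.
; Interacting while held detaches the Cube and re-enables physics.
; An IsAttached flag, set from the attach result, toggles between the two states.
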(event `self.Interact`
  (if (`self.bIsAttached`)
    (`PrimitiveComponent.SetSimulatePhysics` (`self.Cube`) true)
    (`SceneComponent.K2_DetachFromComponent` (`self.Cube`) "KeepWorld" "KeepWorld" "KeepWorld" true)
    (set `self.bIsAttached` false)
    (else
      (bind _asthird_person_character (cast `/Game/ThirdPersonCPP/Blueprints/ThirdPersonCharacter` (`GameplayStatics.GetPlayerCharacter` 0)))
      (`PrimitiveComponent.SetSimulatePhysics` (`self.Cube`) false)
      (bind _returnvalue (`SceneComponent.K2_AttachToComponent` (`self.Cube`) (`/Game/ThirdPersonCPP/Blueprints/ThirdPersonCharacter.HandRef` _asthird_person_character) "None" "KeepWorld" "KeepWorld" "KeepWorld" true))
      (set `self.bIsAttached` _returnvalue))))

(fn `UserConstructionScript`)